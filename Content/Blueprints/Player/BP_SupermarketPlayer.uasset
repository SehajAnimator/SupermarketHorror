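; BP_SupermarketPlayer is the first-person-style player for a supermarket game, handling movement, mouse look, interaction and its HUD.
; WASD and mouse input set stored axis values that Tick applies as movement and controller rotation.
; Each tick also line-traces between two components, storing BPI_FunctionalObject hits and showing their UI; E executes the stored object.
; The stored object is hidden and cleared only when the trace hits nothing.
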(event `self.ReceiveBeginPlay`
  ; Add Player UI
  (bind _returnvalue (`|CreateWidget` "/Game/Blueprints/Player/UW_PlayerHUD.UW_PlayerHUD_C" (`GameplayStatics.GetPlayerController` 0)))
  (bind _output_get (set `self.PlayerUI` _returnvalue))
  (`UserWidget.AddToViewport` _output_get 0))

(event `/Game/Blueprints/Player/BPI_Player.Move`
  (params (`Left/Right` :type "Float (double-precision)") (`Forward/Backward` :type "Float (double-precision)"))
  ; MoveEvent
  (`self.AddMovementInput` (`self.GetActorRightVector`) `Left/Right`)
  (`self.AddMovementInput` (`self.GetActorForwardVector`) `Forward/Backward`))

(event `/Game/Blueprints/Player/BPI_Player.Aim`
  (params (Yaw :type "Float (double-precision)") (Pitch :type "Float (double-precision)"))
  ; AimEvent
  (`self.AddControllerYawInput` Yaw)
  (`self.AddControllerPitchInput` Pitch))

(event `self.ReceiveTick`
  (params (DeltaSeconds :type "Float (single-precision)"))
  ; Update Logic
  (`/Game/Blueprints/Player/BPI_Player.Aim` (`self.Aim_X`) (`self.Aim_Y`))
  (`/Game/Blueprints/Player/BPI_Player.Move` (`self.Move_LR`) (`self.Move_FB`))
  (`self.HandleObjects`))

(event `Key|W`
  (params (Key :type "Key Structure"))
  ; MovementControl
  (:`Pressed`
    (set `self.Move_FB` 1.0))
  (:`Released`
    (set `self.Move_FB` 0.0)))

(event `Key|A`
  (params (Key :type "Key Structure"))
  ; MovementControl
  (:`Pressed`
    (set `self.Move_LR` -1.0))
  (:`Released`
    (set `self.Move_LR` 0.0)))

(event `InputAxisKey|MouseX`
  (params (AxisValue :type "Float (single-precision)"))
  ; AimControl
  (set `self.Aim_X` AxisValue))

(event `Key|S`
  (params (Key :type "Key Structure"))
  ; MovementControl
  (:`Pressed`
    (set `self.Move_FB` -1.0))
  (:`Released`
    (set `self.Move_FB` 0.0)))

(event `Key|D`
  (params (Key :type "Key Structure"))
  ; MovementControl
  (:`Pressed`
    (set `self.Move_LR` 1.0))
  (:`Released`
    (set `self.Move_LR` 0.0)))

(event `InputAxisKey|MouseY`
  (params (AxisValue :type "Float (single-precision)"))
  ; AimControl
  (set `self.Aim_Y` (* AxisValue -1.0)))

(event `Key|E`
  (params (Key :type "Key Structure"))
  (bind _hitobject (`self.HitObject`))
  ; Interaction
  (:`Pressed`
    (if (`KismetSystemLibrary.IsValidInterface` _hitobject)
      (`/Game/Blueprints/InteractableObjects/BPI_FunctionalObject.ExecuteFunction` _hitobject))))

(fn `HandleObjects`
  (bind _hitobject (`self.HitObject`))
  (bind (_outhit _returnvalue) (`KismetSystemLibrary.LineTraceSingle` (`SceneComponent.K2_GetComponentLocation` (`self.Start`)) (`SceneComponent.K2_GetComponentLocation` (`self.End`)) "TraceTypeQuery1"))
  (if _returnvalue
    (bind _asbpi_functional_object (cast `/Game/Blueprints/InteractableObjects/BPI_FunctionalObject` (`.HitActor` (`GameplayStatics.BreakHitResult` _outhit)))
      (:`then`
        (bind _output_get (set `self.HitObject` _asbpi_functional_object))
        (`/Game/Blueprints/InteractableObjects/BPI_FunctionalObject.ShowUI` _output_get))
      (:`CastFailed`
        _))
    (elif (`KismetSystemLibrary.IsValidInterface` _hitobject)
      (`/Game/Blueprints/InteractableObjects/BPI_FunctionalObject.HideUI` _hitobject)
      (set `self.HitObject` null)))
  (return))

(fn `UserConstructionScript`)