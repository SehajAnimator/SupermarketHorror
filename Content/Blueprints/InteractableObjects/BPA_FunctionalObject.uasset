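; BPA_FunctionalObject is an interactable-object actor that carries a name, a description and a UI widget.
; The widget is hidden on BeginPlay, and the ShowUI and HideUI events toggle its visibility.
; GetName and GetDescription return the stored Name and Description values, while the construction script is empty.
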(event `self.ReceiveBeginPlay`
  ; Initial Visibility
  (`SceneComponent.SetVisibility` (`self.Widget`) false false))

(event `/Game/Blueprints/InteractableObjects/BPI_FunctionalObject.ShowUI`
  (`SceneComponent.SetVisibility` (`self.Widget`) true false))

(event `/Game/Blueprints/InteractableObjects/BPI_FunctionalObject.HideUI`
  (`SceneComponent.SetVisibility` (`self.Widget`) false false))

(fn `GetDescription`
  (returns (Value :type String))
  (return (`self.Description`)))

(fn `GetName`
  (returns (Value :type String))
  (return (`self.Name`)))

(fn `UserConstructionScript`)