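; Pickable object actor that exposes a name and description and carries a widget for its in-world prompt.
; On BeginPlay it hides the widget and passes its name to the UW_FunctionalObject inside.
; Events show, hide or reattach the widget, and HandExecuteFunction forwards to the widget's FromExecute.
; OnPickup only checks whether player character 0 is locally controlled and has no pickup logic.
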(event `self.ReceiveBeginPlay`
  ; Init Vis
  (`SceneComponent.SetVisibility` (`self.Widget`) false false)
  ; Change Name
  (bind _asuw_functional_object (cast `/Game/Blueprints/InteractableObjects/UW_FunctionalObject` (`WidgetComponent.GetUserWidgetObject` (`self.Widget`))))
  (`/Game/Blueprints/InteractableObjects/UW_FunctionalObject.SetName` _asuw_functional_object (`self.Name`)))

(event `/Game/Blueprints/PickableObjects/BPI_PickableObject.ShowUI`
  ; UI Vis
  (`SceneComponent.SetVisibility` (`self.Widget`) true false))

(event `/Game/Blueprints/PickableObjects/BPI_PickableObject.HideUI`
  ; UI Vis
  (`SceneComponent.SetVisibility` (`self.Widget`) false false))

(event `/Game/Blueprints/PickableObjects/BPI_PickableObject.SetUIParent`
  (params (Parent :type "SceneComponent Object Reference"))
  ; UI Vis
  (`SceneComponent.K2_AttachToComponent` (`self.Widget`) Parent "None" "KeepRelative" "KeepRelative" "KeepRelative" true))

(event `/Game/Blueprints/PickableObjects/BPI_PickableObject.OnPickup`
  (if (`self.IsLocallyControlled` (`GameplayStatics.GetPlayerCharacter` 0))
    _))

(fn `GetDescription`
  (returns (Description :type String))
  (return (`self.Description`)))

(fn `GetName`
  (returns (Name :type String))
  (return (`self.Name`)))

(fn `HandExecuteFunction`
  (returns (out :type Boolean))
  (bind _asuw_functional_object (cast `/Game/Blueprints/InteractableObjects/UW_FunctionalObject` (`WidgetComponent.GetUserWidgetObject` (`self.Widget`))))
  (`/Game/Blueprints/InteractableObjects/UW_FunctionalObject.FromExecute` _asuw_functional_object)
  (return true))

(fn `UserConstructionScript`)